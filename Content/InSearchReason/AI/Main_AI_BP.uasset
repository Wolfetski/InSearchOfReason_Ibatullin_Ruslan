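; Monster AI pawn that chases the main character on sight and destroys itself once it successfully reaches them.
; PawnSensing triggers AI MoveTo on the seen BP_MainCharacter, while Tick accumulates delta time during movement to play monster footsteps at a fixed interval.
; It also has axis handlers for movement and look, plus an unconnected echolocation timeline that would pulse a material-collection radius and sphere-trace to activate doors and actors.
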(event OnSeePawn(PawnSensing)
  (params (Pawn :type Pawn%20Object%20Reference))
  (bind _asbp_main_character (Utilities|Casting|CastToBP_MainCharacter Pawn))
  (AI|AIMoveTo self "0, 0, 0" _asbp_main_character 1e+02 true
    (:OnSuccess
      (Actor|DestroyActor))))

(event EventTick
  (params (DeltaSeconds :type Float%20%28single-precision%29))
  ;[1 1 1] Звуки Шагов
  (Utilities|FlowControl|Sequence
    (:then_0
      (CallFunction|PlaySoundSteps))))

(event Input|ActionEvents|InputActionInteract
  (params (Key :type Key%20Structure :default "None")))

(event Input|AxisEvents|InputAxisMoveForward
  (params (AxisValue :type Float%20%28single-precision%29))
  ;[1 1 1] Входные данные
  ;;[0.5925 1 0.6093] Движение
  (Pawn|Input|AddMovementInput (Transformation|GetActorForwardVector) AxisValue false))

(event Input|AxisEvents|InputAxisMoveRight
  (params (AxisValue :type Float%20%28single-precision%29))
  ;[1 1 1] Входные данные
  ;;[0.5925 1 0.6093] Движение
  (Pawn|Input|AddMovementInput (Transformation|GetActorRightVector) AxisValue false))

(event Input|AxisEvents|InputAxisTurn
  (params (AxisValue :type Float%20%28single-precision%29))
  ;[1 1 1] Входные данные
  ;;[0.4366 1 0.4713] Поворот
  (Pawn|Input|AddControllerYawInput AxisValue))

(event Input|AxisEvents|InputAxisLookUP
  (params (AxisValue :type Float%20%28single-precision%29))
  ;[1 1 1] Входные данные
  ;;[0.4366 1 0.4713] Поворот
  (Pawn|Input|AddControllerPitchInput AxisValue))

(fn ConstructionScript)

(fn PlaySoundSteps
  (if (> (Math|Vector|VectorLength (Transformation|GetVelocity)) 0.0)
    (Variables|Default|Setcount (+ (Variables|Default|Getcount) (Utilities|Time|GetWorldDeltaSeconds)))
    (if (>= (Variables|Default|Getcount) 0.47)
      (Audio|PlaySoundatLocation "/Game/InSearchReason/Audio/SoundMonster/SoundStepsMonster/SoundStepsMonster.SoundStepsMonster" (Transformation|GetActorLocation) "0, 0, 0" 1.0 1.0 0.0 0 0 0)
      (Variables|Default|Setcount 0.0))
    (else
      (Variables|Default|Setcount 0.0))))