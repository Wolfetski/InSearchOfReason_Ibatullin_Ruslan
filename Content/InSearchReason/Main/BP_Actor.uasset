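; BP_Actor is an actor whose static mesh can be flagged for a timed custom depth effect, such as a post-process highlight.
; Activate turns on custom depth rendering with a non-zero stencil value, waits a few seconds, then calls Deactivate.
; Deactivate switches custom depth off and clears the stencil value.
; Nothing in the Blueprint calls Activate itself, and the construction script is empty.
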(event Custom|Deactivate
  (Rendering|SetRenderCustomDepth (Variables|Default|GetStaticMesh) false)
  (Rendering|SetCustomDepthStencilValue (Variables|Default|GetStaticMesh) 0))

(event Custom|Activate
  (Rendering|SetRenderCustomDepth (Variables|Default|GetStaticMesh) true)
  (Rendering|SetCustomDepthStencilValue (Variables|Default|GetStaticMesh) 1)
  (Utilities|FlowControl|Delay 4.0)
  (CallFunction|Deactivate))

(fn ConstructionScript)