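; BP_Doors is an interactive door that the player opens with the Interact input while inside its Box trigger, which enables and disables the actor's input.
; Pressing plays OpenDoor and a DoorRotation timeline that drives the door's yaw; releasing waits briefly, then plays ClosedDoor and reverses the timeline.
; An Activated event temporarily highlights the meshes through Custom Depth stencil values, then calls Deactivate to reset the stencil.
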(event OnComponentBeginOverlap(Box)
  (params (OverlappedComponent :type Primitive%20Component%20Object%20Reference) (OtherActor :type Actor%20Object%20Reference) (OtherComp :type Primitive%20Component%20Object%20Reference) (OtherBodyIndex :type Integer) (bFromSweep :type Boolean) (SweepResult :type Hit%20Result%20Structure%20%28by%20ref%29))
  ;[1 1 1] Открывание и закрывание двери
  (Input|EnableInput (Game|GetPlayerController 0)))

(event OnComponentEndOverlap(Box)
  (params (OverlappedComponent :type Primitive%20Component%20Object%20Reference) (OtherActor :type Actor%20Object%20Reference) (OtherComp :type Primitive%20Component%20Object%20Reference) (OtherBodyIndex :type Integer))
  ;[1 1 1] Открывание и закрывание двери
  (Input|DisableInput (Game|GetPlayerController 0)))

(event Custom|Activated
  ;[1 1 1] Тригер на локацию
  (Rendering|SetRenderCustomDepth (Variables|Default|GetStaticMesh) true)
  (Rendering|SetCustomDepthStencilValue (Variables|Default|GetStaticMesh) 2)
  (Utilities|FlowControl|Delay 6.5)
  (CallFunction|Deactivate))

(event Custom|Deactivate
  ;[1 1 1] Тригер на локацию
  (Rendering|SetRenderCustomDepth (Variables|Default|GetStaticMesh) true)
  (Rendering|SetCustomDepthStencilValue (Variables|Default|GetStaticMesh) 0))

(event Input|ActionEvents|InputActionInteract
  (params (Key :type Key%20Structure :default "None"))
  ;[1 1 1] Открывание и закрывание двери
  (:Pressed
    (Audio|Components|Audio|Play (Variables|Default|GetOpenDoor) 0.0)
    (bind _doorrotation (Timeline|DoorRotation Play)
      (:Update
        (Transformation|SetRelativeRotation (Variables|Default|GetDoor) (Math|Rotator|MakeRotator 0.0 0.0 _doorrotation) false false))))
  (:Released
    (Utilities|FlowControl|Delay 5.0)
    (Audio|Components|Audio|Play (Variables|Default|GetClosed_Door) 0.0)
    (Timeline|DoorRotation Reverse)))

(fn ConstructionScript)