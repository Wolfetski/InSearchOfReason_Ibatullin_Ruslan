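; Door actor that the player opens and closes with the Interact input, optionally locked behind key 6.
; A box overlap enables and disables the actor's input for the first player controller.
; When NeedAKey is set, it reads Door6HasAKey from a referenced Key_System actor and plays a need-key sound if false.
; Otherwise a FlipFlop alternates playing and reversing a timeline that drives the door's yaw, with open and close sounds.
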(event OnComponentBeginOverlap(Box)
  (params (OverlappedComponent :type Primitive%20Component%20Object%20Reference) (OtherActor :type Actor%20Object%20Reference) (OtherComp :type Primitive%20Component%20Object%20Reference) (OtherBodyIndex :type Integer) (bFromSweep :type Boolean) (SweepResult :type Hit%20Result%20Structure%20%28by%20ref%29))
  (Input|EnableInput (Game|GetPlayerController 0)))

(event OnComponentEndOverlap(Box)
  (params (OverlappedComponent :type Primitive%20Component%20Object%20Reference) (OtherActor :type Actor%20Object%20Reference) (OtherComp :type Primitive%20Component%20Object%20Reference) (OtherBodyIndex :type Integer))
  (Input|DisableInput (Game|GetPlayerController 0)))

(event Input|ActionEvents|InputActionInteract
  (params (Key :type Key%20Structure :default "None"))
  (:Pressed
    (if (Variables|Default|GetNeed_a_key?)
      (bind _askey_system (Utilities|Casting|CastToKey_System (Variables|Default|GetActor)))
      (if (Variables|/Game/InSearchReason/DoorsAndKeys/Key_System.Key_System_C|GetDoor_6_has_a_key _askey_system)
        (Utilities|FlowControl|FlipFlop :!label _label
          (:A
            (Audio|Components|Audio|Play (Variables|Default|GetOpenDoor_Key) 0.0)
            (bind _doorrotation (Timeline|Timeline_0 Play)
              (:Update
                (Transformation|SetRelativeRotation (Variables|Default|GetDoor) (Math|Rotator|MakeRotator 0.0 0.0 _doorrotation) false false))))
          (:B
            (Audio|Components|Audio|Play (Variables|Default|GetClosed_Door) 0.0)
            (Timeline|Timeline_0 Reverse)))
        (else
          (Audio|Components|Audio|Play (Variables|Default|GetNeedKey) 0.0)))
      (else
        (goto _label)))))

(fn ConstructionScript
  (|CallParentFunction))