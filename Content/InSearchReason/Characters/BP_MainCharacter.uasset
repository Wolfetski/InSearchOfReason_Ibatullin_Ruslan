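; BP_MainCharacter is the player character, with axis-driven look and movement plus a scanning ability.
; Pressing Scaning plays a timeline that grows the Radius parameter in the PC_Raadius material parameter collection.
; On each timeline update, a sphere trace around the spring arm scales with the same value and calls Activate on a hit BP_Actor among WorldDynamic objects.
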(event EventBeginPlay)

(event Input|ActionEvents|InputActionInteract
  (params (Key :type Key%20Structure :default "None")))

(event Input|ActionEvents|InputActionScaning
  (params (Key :type Key%20Structure :default "None"))
  (bind _springarm (Variables|Default|GetSpringArm))
  (bind _returnvalue (Transformation|GetWorldLocation _springarm))
  ;[1 1 1] Входные данные
  (:Pressed
    (bind _newtrack_0 (Timeline|Timeline_0 PlayFromStart)
      (:Update
        (Rendering|Material|SetScalarParameterValue "/Game/InSearchReason/Scan/PC_Raadius.PC_Raadius" "Radius" _newtrack_0 :!class /Script/Engine.KismetMaterialLibrary)
        (bind _outhit (Collision|SphereTraceForObjects _returnvalue (+ _returnvalue "0, 0,1.000000") (* _newtrack_0 9e+02) (Utilities|Array|MakeArray "ObjectTypeQuery2") false 0 "None"))
        (bind _asbp_actor (Utilities|Casting|CastToBP_Actor (.hitactor _outhit)))
        (Default|Activate _asbp_actor)))))

(event Input|AxisEvents|InputAxisMoveForward
  (params (AxisValue :type Float%20%28single-precision%29))
  ;[1 1 1] Входные данные
  ;;[0.5925 1 0.6093] Движение
  (Pawn|Input|AddMovementInput (Transformation|GetActorForwardVector) AxisValue false))

(event Input|AxisEvents|InputAxisMoveRight
  (params (AxisValue :type Float%20%28single-precision%29))
  ;[1 1 1] Входные данные
  ;;[0.5925 1 0.6093] Движение
  (Pawn|Input|AddMovementInput (Transformation|GetActorRightVector) AxisValue false))

(event Input|AxisEvents|InputAxisTurn
  (params (AxisValue :type Float%20%28single-precision%29))
  ;[1 1 1] Входные данные
  ;;[0.4366 1 0.4713] Поворот
  (Pawn|Input|AddControllerYawInput AxisValue))

(event Input|AxisEvents|InputAxisLookUP
  (params (AxisValue :type Float%20%28single-precision%29))
  ;[1 1 1] Входные данные
  ;;[0.4366 1 0.4713] Поворот
  (Pawn|Input|AddControllerPitchInput AxisValue))

(fn ConstructionScript)